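; Character audio component that plays walk and run footstep sounds based on the ground surface.
; PlayStep and PlayRunStep trace 200 units down from the mesh owner's location and read the hit physical material's surface type.
; The surface selects a grass, road or dirt sound, with grass as default, spawned attached to the mesh alongside a walk or run movement foley layer.
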(event EventBeginPlay)

(event EventTick
  (params (DeltaSeconds :type Float%20%28single-precision%29)))

(fn PlayStep
  (params (MeshComp :type Mesh%20Component%20Object%20Reference))
  (bind _returnvalue (Components|GetOwner MeshComp))
  (bind _returnvalue_2 (Transformation|GetActorLocation _returnvalue))
  (Utilities|IsValid MeshComp
    (:Is%20Valid
      (bind (_outhit _returnvalue_3) (Collision|LineTraceByChannel _returnvalue_2 (- _returnvalue_2 "0.000000,0.000000,200.000000") "TraceTypeQuery1" false 0 "None"))
      (if _returnvalue_3
        (bind _returnvalue_4 (Audio|SpawnSoundAttached (Utilities|Select :Index (Variables|/Script/PhysicsCore.PhysicalMaterial|GetSurfaceType (.PhysMat (Collision|BreakHitResult _outhit))) :SurfaceType_Default "/Game/Audio/Metasounds/Soundsource/FS_Walk_Grass.FS_Walk_Grass" :SurfaceType1 "/Game/Audio/Metasounds/Soundsource/FS_Walk_Grass.FS_Walk_Grass" :SurfaceType2 "/Game/Audio/Metasounds/Soundsource/FS_Walk_Road.FS_Walk_Road" :SurfaceType3 "/Game/Audio/Metasounds/Soundsource/FS_Walk_Dirt.FS_Walk_Dirt") MeshComp "None" "0, 0, 0" "0, 0, 0" "KeepRelativeOffset" false 1.0 1.0 0.0 0 0))
        (Audio|SpawnSoundAttached "/Game/Audio/Metasounds/Soundsource/FOL_Walk_Mov.FOL_Walk_Mov" MeshComp "None" "0, 0, 0" "0, 0, 0" "KeepRelativeOffset" false 1.0 1.0 0.0 0 0)
        (Audio|Components|Audio|Play _returnvalue_4 0.0)))
    (:Is%20Not%20Valid
      (return))))

(fn PlayRunStep
  (params (NewParam :type Mesh%20Component%20Object%20Reference))
  (bind _returnvalue (Components|GetOwner NewParam))
  (bind _returnvalue_2 (Transformation|GetActorLocation _returnvalue))
  (Utilities|IsValid NewParam
    (:Is%20Valid
      (bind (_outhit _returnvalue_3) (Collision|LineTraceByChannel _returnvalue_2 (- _returnvalue_2 "0.000000,0.000000,200.000000") "TraceTypeQuery1" false 0 "None"))
      (if _returnvalue_3
        (bind _returnvalue_4 (Audio|SpawnSoundAttached (Utilities|Select :Index (Variables|/Script/PhysicsCore.PhysicalMaterial|GetSurfaceType (.PhysMat (Collision|BreakHitResult _outhit))) :SurfaceType_Default "/Game/Audio/Metasounds/Soundsource/FS_Run_Grass.FS_Run_Grass" :SurfaceType1 "/Game/Audio/Metasounds/Soundsource/FS_Run_Grass.FS_Run_Grass" :SurfaceType2 "/Game/Audio/Metasounds/Soundsource/FS_Run_Road.FS_Run_Road" :SurfaceType3 "/Game/Audio/Metasounds/Soundsource/FS_Run_Dirt.FS_Run_Dirt") NewParam "None" "0, 0, 0" "0, 0, 0" "KeepRelativeOffset" false 1.0 1.0 0.0 0 0))
        (Audio|SpawnSoundAttached "/Game/Audio/Metasounds/Soundsource/FOL_Run_Mov.FOL_Run_Mov" NewParam "None" "0, 0, 0" "0, 0, 0" "KeepRelativeOffset" false 1.0 1.0 0.0 0 0)
        (Audio|Components|Audio|Play _returnvalue_4 0.0)))
    (:Is%20Not%20Valid
      (return))))