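; BP_Radio is the radio item, which a player toggles on and off and which plays audio from their radio socket.
; ToggleRadio uses a FlipFlop to spawn a click and the SFX_LP_Radio sound attached to SocketRadio, then click again and stop that sound on the next call.
; RadioInputWidget briefly shows the radio key input hint when the player has the radio equipped.
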(event Custom|Radio%20Input%20Widget
  (params (Player :type BP%20FPS%20Player%20Object%20Reference))
  ;[0.4323 0.04733 0.05972 0.5] Radio Input Widget
  (if (Variables|/Game/LD59/Blueprint/Player/BP_FPS_Player.BP_FPS_Player_C|GetbRadioEquipped Player)
    (Default|ShowHintWidget Player "/Game/LD59/Blueprint/Widgets/RadioKeyInput.RadioKeyInput_C" 7.4)))

(event Custom|ToggleRadio
  (params (OwnerPlayer :type BP%20FPS%20Player%20Object%20Reference))
  (bind _socket_radio (Variables|/Game/LD59/Blueprint/Player/BP_FPS_Player.BP_FPS_Player_C|GetSocket_Radio OwnerPlayer))
  ;[0.107 0.15 0.04092 0.502] Radio Toggle logic
  (Utilities|FlowControl|FlipFlop
    (:A
      ;;[0.8438 0.1184 0.6502 0.5] On/Off sound
      (bind _returnvalue (Audio|SpawnSoundAttached "/Game/Audio/Metasounds/Soundsource/SFX_Radio_Click.SFX_Radio_Click" _socket_radio "None" "0, 0, 0" "0, 0, 0" "KeepRelativeOffset" false 1.0 1.0 0.0 0 0))
      (bind _returnvalue_2 (Audio|SpawnSoundAttached "/Game/Audio/Metasounds/Soundsource/SFX_LP_Radio.SFX_LP_Radio" _socket_radio "None" "0, 0, 0" "0, 0, 0" "KeepRelativeOffset" false 1.0 1.0 0.0 0 0))
      (Audio|Components|Audio|Play _returnvalue_2 0.0))
    (:B
      (Utilities|FlowControl|Sequence
        (:then_0
          (bind _returnvalue_3 (Audio|SpawnSoundAttached "/Game/Audio/Metasounds/Soundsource/SFX_Radio_Click.SFX_Radio_Click" _socket_radio "None" "0, 0, 0" "0, 0, 0" "KeepRelativeOffset" false 1.0 1.0 0.0 0 0))
          (Audio|Components|Audio|Play _returnvalue_3 0.0))
        (:then_1
          (Audio|Components|Audio|Stop _returnvalue_2))))))

(fn ConstructionScript
  (|CallParentFunction))