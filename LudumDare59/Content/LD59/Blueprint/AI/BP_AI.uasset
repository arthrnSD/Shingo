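; BP_AI is a scare enemy that runs forward and can jumpscare the player.
; Run takes a mode and sends the AI to a navmesh-projected point ahead, with the A-to-B mode destroying it shortly after.
; The first player overlap with JumpscareContact briefly switches the view to the AI's camera and plays a sound and animation.
; The view then returns to the player and the AI destroys itself.
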(event OnComponentBeginOverlap(Jumpscarecontact)
  (params (OverlappedComponent :type Primitive%20Component%20Object%20Reference) (OtherActor :type Actor%20Object%20Reference) (OtherComp :type Primitive%20Component%20Object%20Reference) (OtherBodyIndex :type Integer) (bFromSweep :type Boolean) (SweepResult :type Hit%20Result%20Structure%20%28by%20ref%29))
  ;[0 0 0 0.5] Jumpscare Logic
  (Utilities|Casting|CastToBP_FPS_Player OtherActor)
  (Utilities|FlowControl|DoOnce false
    (:Completed
      (CallFunction|AiJumpscare))))

(event Custom|Run
  (params (E_TriggerMode :type E_TriggerMode%20Enum :default "NewEnumerator0"))
  ;[0.1456 0.15 0.02785 0.5] Ai Run Function
  (switch Utilities|FlowControl|Switch|SwitchonE_TriggerMode E_TriggerMode
    (:NewEnumerator0
      (AI|AIMoveTo self (.ProjectedLocation (AI|Navigation|ProjectPointtoNavigation (+ (Transformation|GetActorLocation) (* (Transformation|GetActorForwardVector) "3000.000000,3000.000000,3000.000000")) 0 0 "0, 0, 0")) 0 1e+02 false))
    (:NewEnumerator1
      (AI|AIMoveTo self (.ProjectedLocation (AI|Navigation|ProjectPointtoNavigation (+ (Transformation|GetActorLocation) (* (Transformation|GetActorForwardVector) "3000.000000,3000.000000,3000.000000")) 0 0 "0, 0, 0")) 0 1e+02 false
        (:then
          (Utilities|FlowControl|Delay 1.8)
          (Actor|DestroyActor))))))

(event Custom|Ai%20Jumpscare
  ;[0 0 0 0.5] Jumpscare Logic
  (Game|Player|SetViewTargetwithBlend (Game|GetPlayerController 0) (Components|GetOwner (Variables|Default|GetCamera)) 0.0 "VTBlend_Linear" 0.0 false)
  (Utilities|FlowControl|Delay 0.2)
  (Audio|PlaySound2D 0 1.0 1.0 0.0 0 0)
  (Components|Animation|PlayAnimation (Variables|Character|GetMesh) 0 false)
  (Utilities|FlowControl|Delay 0.0)
  (Game|Player|SetViewTargetwithBlend (Game|GetPlayerController 0) (Game|GetPlayerCharacter 0) 0.0 "VTBlend_Linear" 0.0 false)
  (Actor|GetActorOfClass "/Game/LD59/Blueprint/Player/BP_FPS_Player.BP_FPS_Player_C")
  (Physics|SetSimulatePhysics (Variables|Character|GetMesh) false)
  (Actor|DestroyActor))

(fn ConstructionScript)