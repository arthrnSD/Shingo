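; BP_AISpawner is a one-shot trigger that spawns an enemy or NPC BP_AI when the first-person player enters its Box.
; BeginPlay caches the BP_FPS_Player, and the overlap event passes only that actor through a DoOnce.
; AISpawn creates the AI at the Spawner component's transform, calls Run on it with an enum value, then plays a 2D spawn stinger.
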(event OnComponentBeginOverlap(Box)
  (params (OverlappedComponent :type Primitive%20Component%20Object%20Reference) (OtherActor :type Actor%20Object%20Reference) (OtherComp :type Primitive%20Component%20Object%20Reference) (OtherBodyIndex :type Integer) (bFromSweep :type Boolean) (SweepResult :type Hit%20Result%20Structure%20%28by%20ref%29))
  (if (== OtherActor (Variables|Default|GetAs%20BP%20FPS%20Player))
    (Utilities|FlowControl|DoOnce false
      (:Completed
        (CallFunction|AISpawn)))))

(event Custom|AI%20Spawn
  (bind _spawner (Variables|Default|GetSpawner))
  (Utilities|FlowControl|Sequence
    (:then_0
      (bind _returnvalue (AI|SpawnAIFromClass "/Game/LD59/Blueprint/AI/BP_AI.BP_AI_C" 0 (Transformation|GetWorldLocation _spawner) (Transformation|GetWorldRotation _spawner) false 0))
      (bind _asbp_ai (Utilities|Casting|CastToBP_AI _returnvalue))
      (Default|Run _asbp_ai "NewEnumerator0"))
    (:then_1
      (Audio|PlaySound2D "/Game/Audio/Metasounds/Soundsource/SFX_Stinger_Spawn.SFX_Stinger_Spawn" 1.0 1.0 0.0 0 0))))

(event EventBeginPlay
  (bind _asbp_fps_player (Utilities|Casting|CastToBP_FPS_Player (Game|GetPlayerCharacter 0)))
  (Variables|Default|SetAs%20BP%20FPS%20Player _asbp_fps_player))

(fn ConstructionScript)