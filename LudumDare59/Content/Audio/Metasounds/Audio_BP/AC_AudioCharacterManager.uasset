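; AC_AudioCharacterManager is a character audio component that plays footstep sounds through its PlayStep function.
; PlayStep takes a mesh component and line-traces a short distance down from its owner's location on the Visibility channel.
; On a hit, it selects a sound by the physical material's surface type and spawns it attached to the mesh.
; The surface-to-sound selection shows only an empty default entry.
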(event EventBeginPlay)

(event EventTick
  (params (DeltaSeconds :type Float%20%28single-precision%29)))

(fn PlayStep
  (params (MeshComp :type Mesh%20Component%20Object%20Reference))
  (bind _returnvalue (Components|GetOwner MeshComp))
  (bind _returnvalue_2 (Transformation|GetActorLocation _returnvalue))
  (Utilities|IsValid MeshComp
    (:Is%20Valid
      (bind (_outhit _returnvalue_3) (Collision|LineTraceByChannel _returnvalue_2 (- _returnvalue_2 "0.000000,0.000000,100.000000") "TraceTypeQuery1" false 0 "None"))
      (if _returnvalue_3
        (bind _returnvalue_4 (Audio|SpawnSoundAttached (Utilities|Select :Index (Variables|/Script/PhysicsCore.PhysicalMaterial|GetSurfaceType (.PhysMat (Collision|BreakHitResult _outhit))) :SurfaceType_Default 0) MeshComp "None" "0, 0, 0" "0, 0, 0" "KeepRelativeOffset" false 1.0 1.0 0.0 0 0))
        (Audio|Components|Audio|Play _returnvalue_4 0.0)))
    (:Is%20Not%20Valid
      (return))))